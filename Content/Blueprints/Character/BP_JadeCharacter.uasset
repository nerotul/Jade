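; Player character Blueprint for a team-based shooter, handling HUD, scoreboard, team color and weapon drops.
; Health, inventory and weapon events update a locally created main widget with bars, ammo counts and a burning-ammo icon.
; Holding Tab shows a scoreboard that Tick rebuilds from GameState and PlayerStates while visible.
; Possession picks a team material applied through OnRep, and dropped weapons spawn matching rifle or sniper pickups that keep their magazine ammo.
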(event Custom|ConstructMainWidget
  ;[1 1 1] Main widget construction
  (bind _asfirst_person_anim_bp (Utilities|Casting|CastToFirstPerson_AnimBP (Components|SkeletalMesh|GetAnimInstance (Variables|Default|GetFirstPersonMesh))))
  (Variables|/Game/Assets/FirstPersonArms/Animations/FirstPerson_AnimBP.FirstPerson_AnimBP_C|SetHasRifle _asfirst_person_anim_bp true)
  (if (Pawn|IsLocallyControlled)
    (bind _returnvalue (UserInterface|CreateWidget "/Game/Blueprints/Widgets/WBP_Main.WBP_Main_C"))
    (bind _output_get (Variables|Default|SetMainWidget _returnvalue))
    (UserInterface|Viewport|AddtoViewport _output_get 0)
    (Rendering|Components|TextRender|SetText (Variables|/Game/Blueprints/Widgets/WBP_Main.WBP_Main_C|GetInventoryRifleAmmo (Variables|Default|GetMainWidget)) (Utilities|Text|ToText(Integer) (Variables|/Script/Jade.JadeInventoryComponent|GetInventoryRifleAmmo (Variables|Default|GetCharacterInventory))))
    (Rendering|Components|TextRender|SetText (Variables|/Game/Blueprints/Widgets/WBP_Main.WBP_Main_C|GetInventorySniperAmmo (Variables|Default|GetMainWidget)) (Utilities|Text|ToText(Integer) (Variables|/Script/Jade.JadeInventoryComponent|GetInventorySniperAmmo (Variables|Default|GetCharacterInventory))))
    (CallFunction|UpdateCurrenWeaponAmmo)
    (CallFunction|CreateScoreBoard)))

(event Custom|CreateScoreBoard
  ;[1 1 1] Score board construction and toggling
  (bind _returnvalue (UserInterface|CreateWidget "/Game/Blueprints/Widgets/WBP_ScoreBoard.WBP_ScoreBoard_C"))
  (bind _output_get (Variables|Default|SetScoreWidget _returnvalue))
  (Widget|Panel|AddChild (Variables|/Game/Blueprints/Widgets/WBP_Main.WBP_Main_C|GetScoreBox (Variables|Default|GetMainWidget)) _output_get)
  (Widget|SetVisibility _output_get "Collapsed")
  (CallFunction|UpdateScoreBoard))

(event EventTick
  (params (DeltaSeconds :type Float%20%28single-precision%29))
  (bind _scorewidget (Variables|Default|GetScoreWidget))
  ;[1 1 1] Score board construction and toggling
  (Utilities|IsValid _scorewidget
    (:Is%20Valid
      (if (and (Widget|IsVisible _scorewidget) (Pawn|IsLocallyControlled))
        (CallFunction|UpdateScoreBoard)))))

(event EventOnCharacterDead
  ;[1 1 1] Widget update events
  (if (Pawn|IsLocallyControlled)
    (Widget|SetVisibility (Variables|Default|GetMainWidget) "Collapsed")))

(event EventPossessed
  (params (NewController :type Controller%20Object%20Reference))
  ;[1 1 1] Setting team color
  (bind _asbp_jade_player_state (Utilities|Casting|CastToBP_JadePlayerState (Variables|Default|GetPlayerState)))
  (bind _output_get (Variables|Default|SetAs%20BP%20Jade%20Player%20State _asbp_jade_player_state))
  (if (Utilities|Enum|Equal(Enum) (Variables|/Script/Jade.JadePlayerState|GetPlayerTeam _output_get) "Red")
    (Variables|Default|SetMeshTeamMaterial "/Game/Assets/MI_Solid_Red.MI_Solid_Red")
    (else
      (Variables|Default|SetMeshTeamMaterial "/Game/LevelPrototyping/Materials/MI_Solid_Blue.MI_Solid_Blue"))))

(event EventOnUsingBurningAmmoChanged
  (params (NewState :type Boolean))
  (bind _mainwidget (Variables|Default|GetMainWidget))
  (bind _fireimage (Variables|/Game/Blueprints/Widgets/WBP_Main.WBP_Main_C|GetFireImage _mainwidget))
  ;[1 1 1] Widget update events
  (if (Pawn|IsLocallyControlled)
    (if NewState
      (Widget|SetVisibility _fireimage "Visible")
      (else
        (Widget|SetVisibility _fireimage "Collapsed")))))

(event EventOnDropWeapon
  (params (WeaponDropped :type Jade%20Weapon%20Object%20Reference))
  (bind _returnvalue (Class|JadeWeapon|GetCurrentMagazineAmmo WeaponDropped))
  (bind _returnvalue_2 (Transformation|GetActorForwardVector))
  (bind _returnvalue_3 (Transformation|GetActorLocation))
  (bind _returnvalue_4 (* _returnvalue_2 "200.000000,200.000000,200.000000"))
  (bind _returnvalue_5 (+ _returnvalue_4 _returnvalue_3))
  (bind (_x _y) (Math|Vector|BreakVector _returnvalue_5))
  (bind _returnvalue_6 (Math|Vector|MakeVector _x _y 6e+01))
  (bind _returnvalue_7 (Math|Transform|MakeTransform _returnvalue_6))
  ;[1 1 1] Spawning pickup weapon
  (switch Utilities|FlowControl|Switch|SwitchonEWeaponType (Variables|/Script/Jade.JadeWeapon|GetWeaponType WeaponDropped)
    (:AR
      (bind _returnvalue_8 (Game|SpawnActorfromClass "/Game/Blueprints/Pickups/BP_RiflePickup.BP_RiflePickup_C" _returnvalue_7 "Undefined" "MultiplyWithRoot" 0 0))
      (Class|JadeWeaponPickup|SetMagazineAmmo _returnvalue_8 _returnvalue))
    (:Sniper
      (bind _returnvalue_9 (Game|SpawnActorfromClass "/Game/Blueprints/Pickups/BP_SniperPickup.BP_SniperPickup_C" _returnvalue_7 "Undefined" "MultiplyWithRoot" 0 0))
      (Class|JadeWeaponPickup|SetMagazineAmmo _returnvalue_9 _returnvalue))))

(event EventOnMagazineAmmoChanged
  (params (NewMagazineAmmo :type Float%20%28single-precision%29))
  (bind _mainwidget (Variables|Default|GetMainWidget))
  ;[1 1 1] Widget update events
  (Utilities|IsValid (Variables|Default|GetCurrentWeapon)
    (:Is%20Valid
      (Utilities|IsValid _mainwidget
        (:Is%20Valid
          (Rendering|Components|TextRender|SetText (Variables|/Game/Blueprints/Widgets/WBP_Main.WBP_Main_C|GetTextBlock_CurrentMagazine _mainwidget) (Utilities|Text|ToText(Float) NewMagazineAmmo "HalfToEven")))))))

(event EventOnInventoryRifleAmmoChanged
  (params (NewAmount :type Float%20%28single-precision%29))
  (bind _mainwidget (Variables|Default|GetMainWidget))
  ;[1 1 1] Widget update events
  (Utilities|IsValid (Variables|Default|GetCharacterInventory)
    (:Is%20Valid
      (Utilities|IsValid _mainwidget
        (:Is%20Valid
          (Rendering|Components|TextRender|SetText (Variables|/Game/Blueprints/Widgets/WBP_Main.WBP_Main_C|GetInventoryRifleAmmo _mainwidget) (Utilities|Text|ToText(Float) NewAmount "HalfToEven")))))))

(event EventOnWeaponChanged
  ;[1 1 1] Widget update events
  (CallFunction|UpdateCurrenWeaponAmmo))

(event EventOnArmorChanged
  (params (NewArmor :type Float%20%28single-precision%29))
  (bind _characterhealth (Variables|Default|GetCharacterHealth))
  (bind _mainwidget (Variables|Default|GetMainWidget))
  ;[1 1 1] Widget update events
  (Utilities|IsValid _characterhealth
    (:Is%20Valid
      (Utilities|IsValid _mainwidget
        (:Is%20Valid
          (Progress|SetPercent (Variables|/Game/Blueprints/Widgets/WBP_Main.WBP_Main_C|GetProgressBar_Armor _mainwidget) (/ NewArmor (Class|JadeHealthComponent|GetMaxArmor _characterhealth))))))))

(event EventOnInventorySniperAmmoChanged
  (params (NewAmount :type Float%20%28single-precision%29))
  (bind _mainwidget (Variables|Default|GetMainWidget))
  ;[1 1 1] Widget update events
  (Utilities|IsValid (Variables|Default|GetCharacterInventory)
    (:Is%20Valid
      (Utilities|IsValid _mainwidget
        (:Is%20Valid
          (Rendering|Components|TextRender|SetText (Variables|/Game/Blueprints/Widgets/WBP_Main.WBP_Main_C|GetInventorySniperAmmo _mainwidget) (Utilities|Text|ToText(Float) NewAmount "HalfToEven")))))))

(event EventOnHealthChanged
  (params (NewHealth :type Float%20%28single-precision%29))
  (bind _mainwidget (Variables|Default|GetMainWidget))
  (bind _characterhealth (Variables|Default|GetCharacterHealth))
  ;[1 1 1] Widget update events
  (Utilities|IsValid _characterhealth
    (:Is%20Valid
      (Utilities|IsValid _mainwidget
        (:Is%20Valid
          (Progress|SetPercent (Variables|/Game/Blueprints/Widgets/WBP_Main.WBP_Main_C|GetProgressBar_Health _mainwidget) (/ NewHealth (Class|JadeHealthComponent|GetMaxHealth _characterhealth))))))))

(event Input|KeyboardEvents|Tab
  (params (Key :type Key%20Structure :default "None"))
  (bind _scorewidget (Variables|Default|GetScoreWidget))
  ;[1 1 1] Score board construction and toggling
  (:Pressed
    (Widget|SetVisibility _scorewidget "Visible"))
  (:Released
    (Widget|SetVisibility _scorewidget "Collapsed")))

(fn ConstructionScript)

(fn OnRepMeshTeamMaterial
  (Rendering|Material|SetMaterial (Variables|Character|GetMesh) 0 (Variables|Default|GetMeshTeamMaterial)))

(fn UpdateCurrenWeaponAmmo
  (bind _currentweapon (Variables|Default|GetCurrentWeapon))
  (bind _mainwidget (Variables|Default|GetMainWidget))
  (Utilities|IsValid _currentweapon
    (:Is%20Valid
      (Utilities|IsValid _mainwidget
        (:Is%20Valid
          (Rendering|Components|TextRender|SetText (Variables|/Game/Blueprints/Widgets/WBP_Main.WBP_Main_C|GetTextBlock_CurrentMagazine _mainwidget) (Utilities|Text|ToText(Integer) (Class|JadeWeapon|GetCurrentMagazineAmmo _currentweapon)))
          (Rendering|Components|TextRender|SetText (Variables|/Game/Blueprints/Widgets/WBP_Main.WBP_Main_C|GetTextBlock_MaxMagazine _mainwidget) (Utilities|Text|ToText(Integer) (Class|JadeWeapon|GetMaxMagazineAmmo _currentweapon)))
          (Widget|SetVisibility (Variables|/Game/Blueprints/Widgets/WBP_Main.WBP_Main_C|GetFireImage _mainwidget) "Collapsed"))))))

(fn UpdateScoreBoard
  (bind _scorewidget (Variables|Default|GetScoreWidget))
  (bind _scorewidget_2 (Variables|Default|GetScoreWidget))
  (bind _asbp_jade_game_state (Utilities|Casting|CastToBP_JadeGameState (Game|GetGameState)))
  (Rendering|Components|TextRender|SetText (Variables|/Game/Blueprints/Widgets/WBP_ScoreBoard.WBP_ScoreBoard_C|GetBlueScore _scorewidget_2) (Utilities|Text|ToText(Integer) (Variables|/Script/Jade.JadeGameState|GetBlueTeamScore _asbp_jade_game_state)))
  (Rendering|Components|TextRender|SetText (Variables|/Game/Blueprints/Widgets/WBP_ScoreBoard.WBP_ScoreBoard_C|GetRedScore _scorewidget_2) (Utilities|Text|ToText(Integer) (Variables|/Script/Jade.JadeGameState|GetRedTeamScore _asbp_jade_game_state)))
  (Widget|Panel|ClearChildren (Variables|/Game/Blueprints/Widgets/WBP_ScoreBoard.WBP_ScoreBoard_C|GetRedPlayersBox _scorewidget))
  (Widget|Panel|ClearChildren (Variables|/Game/Blueprints/Widgets/WBP_ScoreBoard.WBP_ScoreBoard_C|GetBluePlayersBox _scorewidget))
  (for _array_element (Variables|/Script/Engine.GameStateBase|GetPlayerArray (Game|GetGameState))
    (bind _asbp_jade_player_state (Utilities|Casting|CastToBP_JadePlayerState _array_element))
    (bind _returnvalue (UserInterface|CreateWidget "/Game/Blueprints/Widgets/WBP_ScoreLine.WBP_ScoreLine_C"))
    (Rendering|Components|TextRender|SetText (Variables|/Game/Blueprints/Widgets/WBP_ScoreLine.WBP_ScoreLine_C|GetPlayername _returnvalue) (Utilities|Text|ToText(String) (PlayerState|GetPlayerName _asbp_jade_player_state)))
    (Rendering|Components|TextRender|SetText (Variables|/Game/Blueprints/Widgets/WBP_ScoreLine.WBP_ScoreLine_C|GetPlayerScore _returnvalue) (Utilities|Text|ToText(Integer) (Variables|/Script/Jade.JadePlayerState|GetPlayerScore _asbp_jade_player_state)))
    (if (Utilities|Enum|Equal(Enum) (Variables|/Script/Jade.JadePlayerState|GetPlayerTeam _asbp_jade_player_state) "Red")
      (Widget|Panel|AddChild (Variables|/Game/Blueprints/Widgets/WBP_ScoreBoard.WBP_ScoreBoard_C|GetRedPlayersBox (Variables|Default|GetScoreWidget)) _returnvalue)
      (else
        (Widget|Panel|AddChild (Variables|/Game/Blueprints/Widgets/WBP_ScoreBoard.WBP_ScoreBoard_C|GetBluePlayersBox (Variables|Default|GetScoreWidget)) _returnvalue)))))

(fn GetCameraRotation
  (return (Variables|Default|GetCharacterCameraRotation)))