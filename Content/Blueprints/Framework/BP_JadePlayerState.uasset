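; BP_JadePlayerState is a player state Blueprint that shows the end-of-match result screen.
; Its FinishMatch event takes the victorious team, removes all widgets and creates a WBP_MatchFinished widget.
; It compares that team with PlayerTeam to set a draw, victory or defeat message, treating NONE as a draw, then adds the widget to the viewport.
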(event Custom|FinishMatch
  (params (VictoriousTeam :type EPlayerTeam%20Enum :default "Red"))
  (Viewport|RemoveAllWidgets)
  (bind _returnvalue (UserInterface|CreateWidget "/Game/Blueprints/Widgets/WBP_MatchFinished.WBP_MatchFinished_C"))
  (if (Utilities|Enum|Equal(Enum) VictoriousTeam "NONE")
    (Rendering|Components|TextRender|SetText (Variables|/Game/Blueprints/Widgets/WBP_MatchFinished.WBP_MatchFinished_C|GetMatchResultText _returnvalue) "DRAW!")
    (elif (Utilities|Enum|Equal(Enum) VictoriousTeam (Variables|Default|GetPlayerTeam))
      (Rendering|Components|TextRender|SetText (Variables|/Game/Blueprints/Widgets/WBP_MatchFinished.WBP_MatchFinished_C|GetMatchResultText _returnvalue) "VICTORY!")
      (else
        (Rendering|Components|TextRender|SetText (Variables|/Game/Blueprints/Widgets/WBP_MatchFinished.WBP_MatchFinished_C|GetMatchResultText _returnvalue) "DEFEAT!"))))
  (UserInterface|Viewport|AddtoViewport _returnvalue 0))

(event EventBeginPlay)

(fn ConstructionScript)