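; BP_JadeGameInstance is the game instance that handles multiplayer session flow between the main menu and lobby.
; CreateMatch starts a five-connection LAN session and opens LobbyMenu as a listen server, on both the immediate and Success outputs.
; JoinMatch joins a supplied session result.
; BacktoMenu destroys the session and, on success, opens MainMenu and adds a WBP_Menu widget to the viewport.
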(event EventCreateMatch
  (|Session (Game|GetPlayerController 0) 5 true true
    (:then
      _)
    (:OnSuccess
      _))
  (Game|OpenLevel(byName) "LobbyMenu" true "listen"))

(event EventJoinMatch
  (params (Session :type Blueprint%20Session%20Result%20Structure))
  (|JoinSession (Game|GetPlayerController 0) Session))

(event EventBacktoMenu
  (|DestroySession (Game|GetPlayerController 0)
    (:OnSuccess
      (Game|OpenLevel(byName) "MainMenu")
      (bind _returnvalue (UserInterface|CreateWidget "/Game/Blueprints/Widgets/WBP_Menu.WBP_Menu_C" (Game|GetPlayerController 0)))
      (UserInterface|Viewport|AddtoViewport _returnvalue 0))))