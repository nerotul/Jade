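; Game mode for a timed Red versus Blue team match that handles player spawning, respawning and the result.
; PostLogin sets each player's team from an incrementing test index, leaving the GameInstance team lookup unused.
; Login and RespawnCharacter spawn a BP_JadeCharacter at the team-named player start, possess it and build its widget.
; A BeginPlay timer calls FinishMatch, which compares GameState scores, sets the winner or a tie and flags completion.
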(event EventRespawnCharacter
  (params (InController :type Controller%20Object%20Reference) (InCharacterTeam :type EPlayerTeam%20Enum :default "Red"))
  (bind _returnvalue (Game|SpawnActorfromClass "/Game/Blueprints/Character/BP_JadeCharacter.BP_JadeCharacter_C" (Transformation|GetActorTransform (Class|GameModeBase|FindPlayerStart InController (Utilities|String|EnumtoString InCharacterTeam))) "Undefined" "MultiplyWithRoot" InController 0))
  (Pawn|Possess InController _returnvalue)
  (Default|ConstructMainWidget _returnvalue))

(event EventBeginPlay
  (Utilities|Time|SetTimerbyFunctionName 0 "FinishMatch" (Variables|Default|GetMatchTime)))

(event EventPostLogin
  (params (NewPlayer :type Player%20Controller%20Object%20Reference))
  (CallFunction|LazyCasttoGameInstance)
  (bind _asbp_jade_player_state (Utilities|Casting|CastToBP_JadePlayerState (Variables|/Script/Engine.Controller|GetPlayerState NewPlayer)))
  (bind _output_get (Variables|/Script/Jade.JadePlayerState|SetPlayerTeam _asbp_jade_player_state (Utilities|Enum|ByteToEnumEPlayerTeam (Math|Conversions|ToByte(Integer) (Variables|Default|GetTestTeamIndex)))))
  (bind _returnvalue (Game|SpawnActorfromClass "/Game/Blueprints/Character/BP_JadeCharacter.BP_JadeCharacter_C" (Transformation|GetActorTransform (Class|GameModeBase|FindPlayerStart NewPlayer (Utilities|String|EnumtoString _output_get))) "Undefined" "MultiplyWithRoot" NewPlayer 0))
  (Pawn|Possess NewPlayer _returnvalue)
  (Default|ConstructMainWidget _returnvalue)
  (Math|Integer|IncrementInt (Variables|Default|GetTestTeamIndex)))

(fn ConstructionScript)

(fn LazyCasttoGameInstance
  (if (== (Variables|Default|GetAs%20BP%20Jade%20Game%20Instance) 0)
    (bind _asbp_jade_game_instance (Utilities|Casting|CastToBP_JadeGameInstance (Game|GetGameInstance)))
    (Variables|Default|SetAs%20BP%20Jade%20Game%20Instance _asbp_jade_game_instance))
  (return))

(fn FinishMatch
  (bind _asbp_jade_game_state (Utilities|Casting|CastToBP_JadeGameState (Game|GetGameState)))
  (if (== (Variables|/Script/Jade.JadeGameState|GetRedTeamScore _asbp_jade_game_state) (Variables|/Script/Jade.JadeGameState|GetBlueTeamScore _asbp_jade_game_state))
    (Variables|/Game/Blueprints/Framework/BP_JadeGameState.BP_JadeGameState_C|SetVictoriousTeam _asbp_jade_game_state "NONE")
    (elif (> (Variables|/Script/Jade.JadeGameState|GetRedTeamScore _asbp_jade_game_state) (Variables|/Script/Jade.JadeGameState|GetBlueTeamScore _asbp_jade_game_state))
      (Variables|/Game/Blueprints/Framework/BP_JadeGameState.BP_JadeGameState_C|SetVictoriousTeam _asbp_jade_game_state "Red")
      (else
        (Variables|/Game/Blueprints/Framework/BP_JadeGameState.BP_JadeGameState_C|SetVictoriousTeam _asbp_jade_game_state "Blue"))))
  (Variables|/Game/Blueprints/Framework/BP_JadeGameState.BP_JadeGameState_C|SetbHasMatchFinished _asbp_jade_game_state true))