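; Lobby game mode that tracks joining players and moves them into the match on JadeMap.
; PostLogin collects each BP_LobbyPlayerState into an array.
; StartMatch copies every player's team into the game instance's PlayerTeams map, keyed by the player state's object display name, so teams persist through travel.
; It then runs a servertravel console command on the first player controller.
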(event Custom|StartMatch
  (CallFunction|SavePlayerTeamforTraveling)
  (Development|ExecuteConsoleCommand "servertravel JadeMap" (Game|GetPlayerController 0)))

(event EventBeginPlay)

(event EventTick
  (params (DeltaSeconds :type Float%20%28single-precision%29)))

(event EventPostLogin
  (params (NewPlayer :type Player%20Controller%20Object%20Reference))
  (bind _asbp_lobby_player_state (Utilities|Casting|CastToBP_LobbyPlayerState (Variables|/Script/Engine.Controller|GetPlayerState NewPlayer)))
  (Utilities|Array|Add (Variables|Default|GetLobbyPlayerStates) _asbp_lobby_player_state))

(fn ConstructionScript)

(fn SavePlayerTeamforTraveling
  (bind _asbp_jade_game_instance (Utilities|Casting|CastToBP_JadeGameInstance (Game|GetGameInstance)))
  (for _array_element (Variables|Default|GetLobbyPlayerStates)
    (Utilities|Map|Add (Variables|/Game/Blueprints/Framework/BP_JadeGameInstance.BP_JadeGameInstance_C|GetPlayerTeams _asbp_jade_game_instance) (Utilities|GetDisplayName _array_element) (Math|Conversions|ToInteger(Byte) (Variables|/Script/Jade.JadePlayerState|GetPlayerTeam _array_element)))))