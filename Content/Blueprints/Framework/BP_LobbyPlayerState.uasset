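; Lobby player state that stores a player's team and manages the lobby menu widget.
; On BeginPlay with authority, a valid local controller gets the Red team through ServerSetTeam, the WBP_Lobby menu and a visible mouse cursor.
; While the menu exists, Tick clears and rebuilds its player list every frame from the game state's PlayerArray.
; EndPlay removes the menu from its parent.
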(event Custom|ServerSetTeam
  (params (Player%20Team :type EPlayerTeam%20Enum :default "Red"))
  (Variables|Default|SetPlayerTeam Player%20Team))

(event Custom|StartWidgetConstruction
  (bind _returnvalue (Game|GetPlayerController))
  (Utilities|IsValid _returnvalue
    (:Is%20Valid
      (if (Pawn|IsLocalController _returnvalue)
        (CallFunction|ServerSetTeam "Red")
        (bind _returnvalue_2 (UserInterface|CreateWidget "/Game/Blueprints/Widgets/WBP_Lobby.WBP_Lobby_C" _returnvalue))
        (bind _output_get (Variables|Default|SetLobbyMenu _returnvalue_2))
        (UserInterface|Viewport|AddtoViewport _output_get 0)
        (Variables|/Script/Engine.PlayerController|SetbShowMouseCursor (Game|GetPlayerController) true)))))

(event EventBeginPlay
  (Networking|SwitchHasAuthority
    (:Authority
      (CallFunction|StartWidgetConstruction))))

(event EventEndPlay
  (params (EndPlayReason :type EEndPlayReason%20Enum :default "Destroyed"))
  (bind _lobbymenu (Variables|Default|GetLobbyMenu))
  (Utilities|IsValid _lobbymenu
    (:Is%20Valid
      (Widget|RemovefromParent _lobbymenu))))

(event EventTick
  (params (DeltaSeconds :type Float%20%28single-precision%29))
  (bind _lobbymenu (Variables|Default|GetLobbyMenu))
  (Utilities|IsValid _lobbymenu
    (:Is%20Valid
      (Widget|Panel|ClearChildren (Variables|/Game/Blueprints/Widgets/WBP_Lobby.WBP_Lobby_C|GetPlayersBox _lobbymenu))
      (for (_ _array_index) (Variables|/Script/Engine.GameStateBase|GetPlayerArray (Game|GetGameState))
        (Default|UpdatePlayerList (Variables|Default|GetLobbyMenu) _array_index)))))

(fn ConstructionScript)